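; Paper character Blueprint that constrains its camera's world position, with special handling for the boss fight level.
; Every Tick it sets the camera's world Z to a fixed offset value and keeps the current Y.
; In the BossFight level, X is also locked to a constant stored on BeginPlay, while other levels keep the camera's current X.
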(event `self.ReceiveBeginPlay`
  (set `self.BossFightLevelName` "BossFight")
  (bind _returnvalue (`GameplayStatics.GetCurrentLevelName` true))
  (if (`KismetStringLibrary.EqualEqual_StrStr` _returnvalue (`self.BossFightLevelName`))
    (set `self.xPos` (`self.cameraXConstantPosOnLastLevel`))))

(event `self.ReceiveTick`
  (params (DeltaSeconds :type "Float (single-precision)"))
  (bind _camera (`self.Camera`))
  (bind _camera_2 (`self.Camera`))
  (bind _returnvalue (`GameplayStatics.GetCurrentLevelName` true))
  (if (`KismetStringLibrary.EqualEqual_StrStr` _returnvalue (`self.BossFightLevelName`))
    (`SceneComponent.K2_SetWorldLocation` _camera (`KismetMathLibrary.MakeVector` (`self.xPos`) (.y (`SceneComponent.K2_GetComponentLocation` _camera)) (`self.cameraZpositionOffset`)) false false)
    (else
      (`SceneComponent.K2_SetWorldLocation` _camera_2 (`KismetMathLibrary.MakeVector` (.x (`SceneComponent.K2_GetComponentLocation` _camera_2)) (.y (`SceneComponent.K2_GetComponentLocation` _camera_2)) (`self.cameraZpositionOffset`)) false false))))

(fn `UserConstructionScript`)